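; Turret tower that tracks and shoots at a SkeletalMeshActor inside its Colission volume.
; Overlap begin stores the target and opens a gate on Tick; any such actor leaving closes it.
; While open, Cabeza turns in yaw and Acoplador adds pitch via RInterpTo, using a fixed DeltaTime rather than frame time.
; SpawnProjectile then fires a FirstPersonProjectile from the ProjectileSpawn transform, throttled by FireDelay.
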(event `self.ReceiveTick`
  (params (DeltaSeconds :type "Float (single-precision)"))
  (bind _cabeza (`self.Cabeza`))
  (bind _turret_rot_speed (`self.turret_rot_speed`))
  (bind _acoplador (`self.Acoplador`))
  (`/Engine/EditorBlueprintResources/StandardMacros.Gate` true :!label _label
    (:`Exit`
      (bind _returnvalue (`SceneComponent.K2_GetComponentLocation` (`SkeletalMeshActor.SkeletalMeshComponent` (stale `self.colission.OnComponentBeginOverlap` _asskeletal_mesh_actor))))
      (bind _roll (.roll (`KismetMathLibrary.RInterpTo` (`SceneComponent.K2_GetComponentRotation` _cabeza) (`KismetMathLibrary.FindLookAtRotation` (`SceneComponent.K2_GetComponentLocation` _cabeza) _returnvalue) 1.0 _turret_rot_speed)))
      (bind _yaw (.yaw (`KismetMathLibrary.RInterpTo` (`SceneComponent.K2_GetComponentRotation` _cabeza) (`KismetMathLibrary.FindLookAtRotation` (`SceneComponent.K2_GetComponentLocation` _cabeza) _returnvalue) 1.0 _turret_rot_speed)))
      (`SceneComponent.K2_SetWorldRotation` (`self.Cabeza`) (`KismetMathLibrary.MakeRotator` _roll 0.0 _yaw) false false)
      (`SceneComponent.K2_SetWorldRotation` (`self.Acoplador`) (`KismetMathLibrary.MakeRotator` _roll (.pitch (`KismetMathLibrary.RInterpTo` (`SceneComponent.K2_GetComponentRotation` _acoplador) (`KismetMathLibrary.FindLookAtRotation` (`SceneComponent.K2_GetComponentLocation` _acoplador) _returnvalue) 1.0 _turret_rot_speed)) _yaw) false false)
      (`self.SpawnProjectile`))))

(event `self.colission.OnComponentBeginOverlap`
  (params (OverlappedComponent :type "PrimitiveComponent Object Reference") (OtherActor :type "Actor Object Reference") (OtherComp :type "PrimitiveComponent Object Reference") (OtherBodyIndex :type Integer) (bFromSweep :type Boolean) (SweepResult :type "HitResult Structure (by ref)"))
  (if (`KismetMathLibrary.ClassIsChildOf` (`GameplayStatics.GetObjectClass` OtherActor) "/Script/Engine.SkeletalMeshActor")
    (bind _asskeletal_mesh_actor (cast `SkeletalMeshActor` OtherActor))
    (goto _label :!via `Open`)))

(event `self.colission.OnComponentEndOverlap`
  (params (OverlappedComponent :type "PrimitiveComponent Object Reference") (OtherActor :type "Actor Object Reference") (OtherComp :type "PrimitiveComponent Object Reference") (OtherBodyIndex :type Integer))
  (if (`KismetMathLibrary.ClassIsChildOf` (`GameplayStatics.GetObjectClass` OtherActor) "/Script/Engine.SkeletalMeshActor")
    (cast `SkeletalMeshActor` OtherActor)
    (goto _label :!via `Close`)))

(fn `SpawnProjectile`
  (bind _returnvalue (`KismetSystemLibrary.GetGameTimeInSeconds`))
  (if (> _returnvalue (`self.game_time_fire`))
    (set `self.game_time_fire` (+ _returnvalue (`self.fire_delay`)))
    (`|SpawnActorFromClass` "/Game/Assets/Blueprints/FirstPersonProjectile.FirstPersonProjectile_C" (`SceneComponent.K2_GetComponentToWorld` (`self.projectile_spawn`)) "Undefined" "OverrideRootScale")))

(fn `UserConstructionScript`)