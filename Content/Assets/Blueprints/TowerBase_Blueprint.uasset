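; TowerBase is a clickable tower build spot that opens a tower menu and hosts the built tower.
; Clicking it spawns MenuTower_Blueprint slightly raised on the base and stores it as Menu.
; CrearTorre, not called within this Blueprint, detaches and destroys that menu, then spawns and stores the Tower.
; A shared Spawn helper attaches each new actor to the base with KeepRelative rules, so spawn transforms act as local offsets.
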(event `self.ReceiveActorOnClicked`
  (params (ButtonPressed :type "Key Structure" :default "AnyKey"))
  ;[1 1 1] Crear menú de torres
  (bind _objeto (`self.Spawn` "/Game/Assets/Blueprints/MenuTower_Blueprint.MenuTower_Blueprint_C" (`KismetMathLibrary.MakeTransform` (0.0 0.0 20.0))))
  (set `self.menu` _objeto))

(fn `crearTorre`
  (bind _menu (`self.menu`))
  ;[1 1 1] Quitar menú
  (`self.K2_DetachFromActor` _menu "KeepRelative" "KeepRelative" "KeepRelative")
  (`self.K2_DestroyActor` _menu)
  ;[1 1 1] Crear torre
  (bind _objeto (`self.Spawn` "/Game/Assets/Blueprints/Tower.Tower_C" (`KismetMathLibrary.MakeTransform` (0.0 0.0 0.0))))
  (set `self.tower` _objeto))

(fn `Spawn`
  (params (Clase :type "Actor Class Reference") (Transformacion :type "Transform Structure"))
  (returns (Objeto :type "Actor Object Reference"))
  (bind _returnvalue (`|SpawnActorFromClass` Clase Transformacion "Undefined" "OverrideRootScale"))
  (`self.K2_AttachToActor` _returnvalue self "None" "KeepRelative" "KeepRelative" "KeepRelative" true)
  (return _returnvalue))

(fn `UserConstructionScript`)