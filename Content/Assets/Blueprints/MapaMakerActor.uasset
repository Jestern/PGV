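; MapaMakerActor is an actor that holds game resources (Recursos) and the current wave number (OleadaActual), apparently for a build-and-waves mode.
; PuedoConstruir checks whether a cost is affordable, while other functions add resources, subtract costs and advance the wave.
; Resource changes use by-reference Increment and Decrement helpers, and spending prints the result.
; It has no active event or construction logic, so its functions rely on external callers.
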(fn `DecrementarRecursos`
  (params (Coste :type Integer))
  (bind ___value (`self.Decrement` (`self.Recursos`) Coste)
    (:`  `
      (`KismetSystemLibrary.PrintString` (`KismetStringLibrary.Conv_IntToString` ___value)))))

(fn `IncrementarOleada`
  (`/Engine/EditorBlueprintResources/StandardMacros.IncrementInt` (`self.OleadaActual`)))

(fn `IncrementarRecursos`
  (params (Recursos :type Integer))
  (`self.Increment` (`self.Recursos`) Recursos))

(fn `PuedoConstruir`
  (params (Coste :type Integer))
  (returns (Construir :type Boolean))
  (return (<= Coste (`self.Recursos`))))

(fn `UserConstructionScript`)