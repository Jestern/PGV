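; MenuBuild is the build menu actor for a tower base, offering a tower option and a cancel option.
; On BeginPlay it spawns MenuTower_Blueprint and MenuCancel at opposite X offsets through a Spawn helper that attaches them to itself.
; CrearTorre and QuitarMenu find the owning TowerBase_Blueprint through the root component's attach parent and forward tower creation, with its price, and menu removal to it.
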(event `self.ReceiveBeginPlay`
  (bind _objeto (`self.Spawn` "/Game/Assets/Blueprints/MenuTower_Blueprint.MenuTower_Blueprint_C" (`KismetMathLibrary.MakeTransform` (-90.0 0.0 0.0))))
  (set `self.MenuTower` _objeto)
  (bind _objeto_2 (`self.Spawn` "/Game/Assets/Blueprints/MenuCancel.MenuCancel_C" (`KismetMathLibrary.MakeTransform` (90.0 0.0 0.0))))
  (set `self.MenuCancel` _objeto_2))

(fn `CrearTorre`
  (params (PrecioTorre :type Integer))
  (bind _astower_base_blueprint (cast `/Game/Assets/Blueprints/TowerBase_Blueprint` (`ActorComponent.GetOwner` (`SceneComponent.GetAttachParent` (`self.K2_GetRootComponent`)))))
  (`/Game/Assets/Blueprints/TowerBase_Blueprint.crearTorre` _astower_base_blueprint PrecioTorre))

(fn `QuitarMenu`
  (bind _astower_base_blueprint (cast `/Game/Assets/Blueprints/TowerBase_Blueprint` (`ActorComponent.GetOwner` (`SceneComponent.GetAttachParent` (`self.K2_GetRootComponent`)))))
  (`/Game/Assets/Blueprints/TowerBase_Blueprint.QuitarMenu` _astower_base_blueprint))

(fn `Spawn`
  (params (Clase :type "Actor Class Reference") (Transformacion :type "Transform Structure"))
  (returns (Objeto :type "Actor Object Reference"))
  (bind _returnvalue (`|SpawnActorFromClass` Clase Transformacion "Undefined" "OverrideRootScale"))
  (`self.K2_AttachToActor` _returnvalue self "None" "KeepRelative" "KeepRelative" "KeepRelative" true)
  (return _returnvalue))

(fn `UserConstructionScript`)