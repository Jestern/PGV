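; Enemy that walks along a Route spline, attacks on overlap with Base or a "Cuerpo" component, and dies from projectile hits.
; Tick advances a frame-based spline distance, which the Movement timeline turns into location and yaw-corrected rotation.
; Collider overlaps set Attack or Idle to halt movement, with idling on "CajaBicho" contact only after first placement.
; Projectiles deal random damage; death plays an animation, then destroys the actor.
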(event `self.ReceiveTick`
  (params (DeltaSeconds :type "Float (single-precision)"))
  (if (and (and (not (`self.Attack`)) (not (`self.Idle`))) (> (`self.Salud`) 0))
    (set `self.EnemyDistance` (+ (`self.EnemyDistance`) 5.0))))

(event `self.MyCollider.OnComponentBeginOverlap`
  (params (OverlappedComponent :type "PrimitiveComponent Object Reference") (OtherActor :type "Actor Object Reference") (OtherComp :type "PrimitiveComponent Object Reference") (OtherBodyIndex :type Integer) (bFromSweep :type Boolean) (SweepResult :type "HitResult Structure (by ref)"))
  (if (`self.Death`)
    _
    (elif (and (== (`GameplayStatics.GetObjectClass` OtherActor) "/Game/Assets/Blueprints/FirstPersonProjectile.FirstPersonProjectile_C") (> (`self.Salud`) 0))
      (set `self.Salud` (- (`self.Salud`) (`KismetMathLibrary.RandomIntegerInRange` 10 30)))
      (if (<= (`self.Salud`) 0)
        (set `self.Death` true)
        (`SkeletalMeshComponent.PlayAnimation` (`self.SkeletalMeshComponent`) (`self.DeathAnimation`) false)
        (`KismetSystemLibrary.Delay` 2.0)
        (`self.K2_DestroyActor`))
      (elif (or (`KismetStringLibrary.EqualEqual_StrStr` (`KismetSystemLibrary.GetObjectName` OtherComp) "Cuerpo") (== (`GameplayStatics.GetObjectClass` OtherActor) "/Game/Assets/Blueprints/Base.Base_C"))
        (set `self.Attack` true)
        (`SkeletalMeshComponent.PlayAnimation` (`self.SkeletalMeshComponent`) (`self.AttackAnimation`) true)
        (elif (and (and (`KismetStringLibrary.EqualEqual_StrStr` (`KismetSystemLibrary.GetObjectName` OtherComp) "CajaBicho") (`self.Spawn`)) (not (`self.Attack`)))
          (set `self.Idle` true)
          (`SkeletalMeshComponent.PlayAnimation` (`self.SkeletalMeshComponent`) (`self.IdleAnimation`) true))))))

(event `self.ReceiveBeginPlay`
  (bind _route (`self.Route`))
  (`SkeletalMeshComponent.PlayAnimation` (`self.SkeletalMeshComponent`) (`self.WalkAnimation`) true)
  (`Timeline|Movement`
    (:`Update`
      (if (and (`KismetSystemLibrary.IsValid` _route) (`KismetMathLibrary.BooleanNOR` (`self.Attack`) (`self.Idle`)))
        (`self.K2_SetActorLocationAndRotation` (`SplineComponent.GetLocationAtDistanceAlongSpline` (`/Game/Assets/Blueprints/SplineBP.Spline` _route) (`self.EnemyDistance`) "World") (`KismetMathLibrary.ComposeRotators` (`SplineComponent.GetRotationAtDistanceAlongSpline` (`/Game/Assets/Blueprints/SplineBP.Spline` (`self.Route`)) (`self.EnemyDistance`) "World") (struct :`Yaw` -90.0)))
        (`/Engine/EditorBlueprintResources/StandardMacros.DoOnce` false
          (:`Completed`
            (set `self.Spawn` true)))))))

(event `self.MyCollider.OnComponentEndOverlap`
  (params (OverlappedComponent :type "PrimitiveComponent Object Reference") (OtherActor :type "Actor Object Reference") (OtherComp :type "PrimitiveComponent Object Reference") (OtherBodyIndex :type Integer))
  (if (`self.Death`)
    _
    (elif (or (`KismetStringLibrary.EqualEqual_StrStr` (`KismetSystemLibrary.GetObjectName` OtherComp) "Cuerpo") (== (`GameplayStatics.GetObjectClass` OtherActor) "/Game/Assets/Blueprints/Base.Base_C"))
      (set `self.Attack` false)
      (set `self.EnemyDistance` (+ (`self.EnemyDistance`) 5.0))
      (`SkeletalMeshComponent.PlayAnimation` (`self.SkeletalMeshComponent`) (`self.WalkAnimation`) true)
      (elif (`KismetStringLibrary.EqualEqual_StrStr` (`KismetSystemLibrary.GetObjectName` OtherComp) "CajaBicho")
        (set `self.Idle` false)
        (`SkeletalMeshComponent.PlayAnimation` (`self.SkeletalMeshComponent`) (`self.WalkAnimation`) true)))))

(fn `UserConstructionScript`)